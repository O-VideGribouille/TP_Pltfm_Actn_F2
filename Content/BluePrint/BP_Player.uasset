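; Player character Blueprint with camera-relative movement, mouse look, jumping and a camera fade-in on BeginPlay.
; InfligerDegat clamps health, then either opens Dead_Restart at zero or copies the new value to BP_GameInstance.
; Helper functions add to the collectable score, open the next level by indexed name, and shift walk speed or jump velocity through four Cpct presets.
; The UI creation call is disconnected, noted as moved to level Blueprints.
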(event `self.ReceiveBeginPlay`
  (`|ExecutionSequence`
    (:`then_1`
      ;[1 1 1] Transition
      (`PlayerCameraManager.StartCameraFade` :`self` (`GameplayStatics.GetPlayerCameraManager` 0) :`FromAlpha` 1.0 :`Duration` 3.0))))

(event `InputAxis|MoveForward`
  (params (AxisValue :type "Float (single-precision)"))
  ;[1 1 1] Mouvements personnage
  (`self.AddMovementInput` (`SceneComponent.GetForwardVector` (`self.Camera`)) AxisValue))

(event `InputAxis|Turn`
  (params (AxisValue :type "Float (single-precision)"))
  ;[1 1 1] Input de la souris
  (`self.AddControllerYawInput` AxisValue))

(event `InputAxis|LookUp`
  (params (AxisValue :type "Float (single-precision)"))
  ;[1 1 1] Input de la souris
  (`self.AddControllerPitchInput` AxisValue))

(event `InputAxis|MoveRight`
  (params (AxisValue :type "Float (single-precision)"))
  ;[1 1 1] Mouvements personnage
  (`self.AddMovementInput` (`SceneComponent.GetRightVector` (`self.Camera`)) AxisValue))

(event `InputAction|Jump`
  (params (Key :type "Key Structure"))
  ;[1 1 1] Jump (inutilisable Nv1)
  (:`Pressed`
    (`self.Jump`))
  (:`Released`
    (`self.StopJumping`)))

(fn `Cpct_1`
  (bind _charactermovement (`self.CharacterMovement`))
  (bind _charactermovement_2 (`self.CharacterMovement`))
  (`|ExecutionSequence`
    (:`then_0`
      (set `CharacterMovementComponent.JumpZVelocity` (- (`CharacterMovementComponent.JumpZVelocity` _charactermovement_2) 280.0) _charactermovement_2))
    (:`then_1`
      (set `CharacterMovementComponent.MaxWalkSpeed` (- (`CharacterMovementComponent.MaxWalkSpeed` _charactermovement) 400.0) _charactermovement))))

(fn `Cpct_2`
  (bind _charactermovement (`self.CharacterMovement`))
  (set `CharacterMovementComponent.MaxWalkSpeed` (- (`CharacterMovementComponent.MaxWalkSpeed` _charactermovement) 200.0) _charactermovement))

(fn `Cpct_3`
  (bind _charactermovement (`self.CharacterMovement`))
  (set `CharacterMovementComponent.JumpZVelocity` (+ (`CharacterMovementComponent.JumpZVelocity` _charactermovement) 300.0) _charactermovement))

(fn `Cpct_4`
  (bind _charactermovement (`self.CharacterMovement`))
  (bind _charactermovement_2 (`self.CharacterMovement`))
  (`|ExecutionSequence`
    (:`then_0`
      (set `CharacterMovementComponent.JumpZVelocity` (- (`CharacterMovementComponent.JumpZVelocity` _charactermovement_2) 180.0) _charactermovement_2))
    (:`then_1`
      (set `CharacterMovementComponent.MaxWalkSpeed` (- (`CharacterMovementComponent.MaxWalkSpeed` _charactermovement) 520.0) _charactermovement))))

(fn `Increase_Collectable`
  (params (`Score Ttl` :type Integer))
  ;[1 1 1] Incrementation score
  (set `self.Collectables_Score` (+ `Score Ttl` (`self.Collectables_Score`))))

(fn `InfligerDegat`
  (params (PointDegat :type Integer))
  (bind _returnvalue (`KismetMathLibrary.Clamp` (- (`self.Vie`) PointDegat) 0 (`self.VieMax`)))
  (if (== _returnvalue 0)
    (`GameplayStatics.OpenLevel` "Dead_Restart")
    (else
      (bind _output_get (set `self.Vie` _returnvalue))
      ;[1 1 1] donnée les valeurs du personnage au game instance
      (bind _asbp_game_instance (cast `/Game/BluePrint/BP_GameInstance` (`GameplayStatics.GetGameInstance`)))
      (set `/Game/BluePrint/BP_GameInstance.Vie_Player` _output_get _asbp_game_instance))))

(fn `Load_Next_Level`
  ;[1 1 1] Pour passer au niveau suivant
  (`GameplayStatics.OpenLevel` (`|GetArrayItem` (`self.NextLevelName`) (`self.NextLevelPoint`))))

(fn `UserConstructionScript`)