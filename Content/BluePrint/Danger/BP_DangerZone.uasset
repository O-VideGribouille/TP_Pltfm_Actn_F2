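; BP_DangerZone is a hazard actor meant to inflict damage over time on BP_Player.
; Overlapping its Debuff component stores the player and starts a looping 3-second timer.
; Each tick subtracts PointDegat from the player's Vie and increments Compteur while Compteur exceeds Duree, otherwise clearing the timer.
; No end-overlap handling or counter reset appears in the graph.
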(event `Degats`
  ;[1 1 1] Function Timer pour infliger des dégât sur la durée
  (bind _returnvalue (`KismetSystemLibrary.K2_SetTimerDelegate` (delegate `InfligerDegatsT`) 3.0 true)))

(event `InfligerDegatsT`
  ;[1 1 1] Function Timer pour infliger des dégât sur la durée
  (if (> (`self.Compteur`) (`self.Duree`))
    (set `/Game/BluePrint/BP_Player.Vie` (- (`/Game/BluePrint/BP_Player.Vie` (stale `self.Debuff.OnComponentBeginOverlap` _asbp_player)) (`self.PointDegat`)) (stale `self.Debuff.OnComponentBeginOverlap` _asbp_player))
    (`/Engine/EditorBlueprintResources/StandardMacros.IncrementInt` (`self.Compteur`))
    (else
      (`KismetSystemLibrary.K2_ClearAndInvalidateTimerHandle` (stale `Degats` _returnvalue)))))

(event `self.Debuff.OnComponentBeginOverlap`
  (params (OverlappedComponent :type "PrimitiveComponent Object Reference") (OtherActor :type "Actor Object Reference") (OtherComp :type "PrimitiveComponent Object Reference") (OtherBodyIndex :type Integer) (bFromSweep :type Boolean) (SweepResult :type "HitResult Structure (by ref)"))
  (bind _asbp_player (cast `/Game/BluePrint/BP_Player` OtherActor))
  (`self.Degats`))

(fn `UserConstructionScript`)