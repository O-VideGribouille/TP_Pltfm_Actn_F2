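; BP_Ballon is a moving balloon hazard that damages the player on contact.
; The construction script sets an InterpToMovement component to travel between two relative points, LctA and LctB, over a configurable duration.
; When its capsule begins overlapping a BP_Player, it calls that player's InfligerDegat with PointDegat, once per touch.
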(event `self.Capsule.OnComponentBeginOverlap`
  (params (OverlappedComponent :type "PrimitiveComponent Object Reference") (OtherActor :type "Actor Object Reference") (OtherComp :type "PrimitiveComponent Object Reference") (OtherBodyIndex :type Integer) (bFromSweep :type Boolean) (SweepResult :type "HitResult Structure (by ref)"))
  ;[1 1 1] Infliger une fois par touché des dégâts au personnage
  (bind _asbp_player (cast `/Game/BluePrint/BP_Player` OtherActor))
  (`/Game/BluePrint/BP_Player.InfligerDegat` _asbp_player (`self.PointDegat`)))

(fn `UserConstructionScript`
  (bind _interptomovement (`self.InterpToMovement`))
  ;[1 1 1] Déplacement du ballon
  (set `InterpToMovementComponent.ControlPoints` (`|MakeArray` (make `InterpControlPoint` (`self.Lct_A`)) (make `InterpControlPoint` (`self.Lct_B`))) _interptomovement)
  (set `InterpToMovementComponent.Duration` (`self.Duration_mvmnt`) _interptomovement))