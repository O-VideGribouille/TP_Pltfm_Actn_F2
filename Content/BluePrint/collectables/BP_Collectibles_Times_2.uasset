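; BP_Collectibles_Times_2 is a crystal collectible that the player picks up on overlap, adding ScoreDefault to their collectable score.
; On a player overlap, it stores its location and scale, then a timeline lerps it toward the player's current position while shrinking it to zero.
; When the timeline finishes, it destroys itself, calls IncreaseCollectable on BP_Player and copies the score to BP_GameInstance for the next level.
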(event `self.ReceiveActorBeginOverlap`
  (params (OtherActor :type "Actor Object Reference"))
  ;[1 1 1] Récupération de collectable
  ;;[1 1 1] Vérifie s'il s'agit du joueur
  (`self.Is Player` OtherActor
    (:`Is Player`
      ;;[1 0.902 0.2392] Encapsulation 1
      (`self.Store Starting Values`)
      ;;[1 1 1] Animation déplacement collectables
      (bind (_direction _collection_progress) (`Timeline|Alpha Blent Timeline`)
        (:`Update`
          ;;[1 0.902 0.2392] Encaplsulation 2
          (`self.Move To Player` _collection_progress)
          (`self.Scale Crystal` _collection_progress))
        (:`Finished`
          (`self.K2_DestroyActor`)
          ;[1 1 1] Add score + visuel - Avec Game Instence
          (bind _asbp_player (cast `/Game/BluePrint/BP_Player` (`GameplayStatics.GetPlayerCharacter` 0)))
          (`|ExecutionSequence`
            (:`then_0`
              (`/Game/BluePrint/BP_Player.Increase_Collectable` _asbp_player (`self.Score default`)))
            (:`then_1`
              ;;[1 1 1] Récupération Next Level
              (bind _output_get (set `/Game/BluePrint/BP_Player.Collectables_Score` (`/Game/BluePrint/BP_Player.Collectables_Score` _asbp_player) _asbp_player))
              (bind _asbp_game_instance (cast `/Game/BluePrint/BP_GameInstance` (`GameplayStatics.GetGameInstance`)))
              (set `/Game/BluePrint/BP_GameInstance.Collect_Player` _output_get _asbp_game_instance))))))))

(fn `Move To Player`
  (params (Alpha :type "Float (double-precision)"))
  (`self.K2_SetActorLocation` (`KismetMathLibrary.VLerp` (`self.Lerp Start Location`) (`self.K2_GetActorLocation` (`GameplayStatics.GetPlayerPawn` 0)) Alpha)))

(fn `Scale Crystal`
  (params (Alpha :type "Float (double-precision)"))
  (`self.SetActorScale3D` (`KismetMathLibrary.VLerp` (`self.Start Scale`) (0.0 0.0 0.0) Alpha)))

(fn `Store Starting Values`
  (set `self.Lerp Start Location` (`self.K2_GetActorLocation`))
  (set `self.Start Scale` (`self.GetActorScale3D`)))

(fn `UserConstructionScript`)